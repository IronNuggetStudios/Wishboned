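; Pickup component that gives its owning actor effects on the player: changing max health, healing or adding coins.
; SetupPickup stores the owner, while BeingPicked caches the first BP_PlayerCharacter, compares it to the overlapping actor and checks prior use.
; Effect events edit player stats directly and set Used; deduction requires the amount to be at least max health, and healing is unclamped.
; Picked destroys the owner one second later if used.
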(event Custom|Being%20Picked
  (params (Overlapping%20Actor :type Object%20Object%20Reference))
  (CallFunction|IsPlayer? Overlapping%20Actor)
  (CallFunction|HasBeenUsed?))

(event Custom|Setup%20Pickup
  (params (OwningActor :type Actor%20Object%20Reference))
  (Variables|Default|SetOwningActor OwningActor))

(event Custom|Deduct%20Max%20Health
  (params (Health :type Float%20%28single-precision%29))
  (bind _playerref (Variables|Default|GetPlayerRef))
  (if (>= Health (Variables|/Game/Blueprints/Player/BP_PlayerCharacter.BP_PlayerCharacter_C|GetMaxHealth _playerref))
    (Variables|/Game/Blueprints/Player/BP_PlayerCharacter.BP_PlayerCharacter_C|SetCurrentHealth _playerref (- (Variables|/Game/Blueprints/Player/BP_PlayerCharacter.BP_PlayerCharacter_C|GetCurrentHealth _playerref) Health))
    (Variables|/Game/Blueprints/Player/BP_PlayerCharacter.BP_PlayerCharacter_C|SetMaxHealth _playerref (- (Variables|/Game/Blueprints/Player/BP_PlayerCharacter.BP_PlayerCharacter_C|GetMaxHealth _playerref) Health))
    (Variables|Default|SetUsed true)))

(event Custom|Heal%20%20Health
  (params (Health :type Float%20%28single-precision%29))
  (bind _playerref (Variables|Default|GetPlayerRef))
  (if (< (Variables|/Game/Blueprints/Player/BP_PlayerCharacter.BP_PlayerCharacter_C|GetCurrentHealth _playerref) (Variables|/Game/Blueprints/Player/BP_PlayerCharacter.BP_PlayerCharacter_C|GetMaxHealth _playerref))
    (Variables|/Game/Blueprints/Player/BP_PlayerCharacter.BP_PlayerCharacter_C|SetCurrentHealth _playerref (+ Health (Variables|/Game/Blueprints/Player/BP_PlayerCharacter.BP_PlayerCharacter_C|GetCurrentHealth _playerref)))
    (Variables|Default|SetUsed true)))

(event Custom|Add%20Max%20Health
  (params (Health :type Float%20%28single-precision%29))
  (bind _playerref (Variables|Default|GetPlayerRef))
  (Variables|/Game/Blueprints/Player/BP_PlayerCharacter.BP_PlayerCharacter_C|SetCurrentHealth _playerref (+ Health (Variables|/Game/Blueprints/Player/BP_PlayerCharacter.BP_PlayerCharacter_C|GetCurrentHealth _playerref)))
  (Variables|/Game/Blueprints/Player/BP_PlayerCharacter.BP_PlayerCharacter_C|SetMaxHealth _playerref (+ Health (Variables|/Game/Blueprints/Player/BP_PlayerCharacter.BP_PlayerCharacter_C|GetMaxHealth _playerref)))
  (Variables|Default|SetUsed true))

(event Custom|Add%20Coins
  (params (Coins :type Integer))
  (bind _playerref (Variables|Default|GetPlayerRef))
  (Variables|/Game/Blueprints/Player/BP_PlayerCharacter.BP_PlayerCharacter_C|SetCoins _playerref (+ Coins (Variables|/Game/Blueprints/Player/BP_PlayerCharacter.BP_PlayerCharacter_C|GetCoins _playerref)))
  (Variables|Default|SetUsed true))

(event Custom|Picked
  (if (Variables|Default|GetUsed)
    (Utilities|FlowControl|Delay 1.0)
    (Actor|DestroyActor (Variables|Default|GetOwningActor))))

(fn HasBeenUsed?
  (if (not (Variables|Default|GetUsed))
    (return)))

(fn IsPlayer?
  (params (B :type Object%20Object%20Reference))
  (bind _outactors (Actor|GetAllActorsOfClass "/Game/Blueprints/Player/BP_PlayerCharacter.BP_PlayerCharacter_C"))
  (bind _output_get (Variables|Default|SetPlayerRef (Utilities|Array|Get(acopy) _outactors)))
  (if (== _output_get B)
    (return)))