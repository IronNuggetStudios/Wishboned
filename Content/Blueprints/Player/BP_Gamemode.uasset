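; Game mode for a local multiplayer game that handles player spawning and progression through an ordered list of room levels.
; On BeginPlay it finds the current level in Rooms to set NextRoom, using "End" after the last.
; Outside the "Start" level, it creates local players and possesses characters spawned at PlayerStarts tagged with each player index.
; RoomComplete opens the next room or shows the game-over widget.
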(event Custom|BreakLoop
  (bind _rooms (Variables|Rooms|GetRooms))
  (bind _returnvalue (Utilities|Array|Length _rooms))
  (bind _returnvalue_2 (- _returnvalue 1))
  (Utilities|Array|ForEachLoopwithBreak _rooms) ; enters at Break
)

(event EventBeginPlay
  (bind _rooms (Variables|Rooms|GetRooms))
  (bind _returnvalue (Utilities|Array|Length _rooms))
  (bind _returnvalue_2 (- _returnvalue 1))
  (Utilities|FlowControl|Sequence
    (:then_0
      (bind _returnvalue_3 (Game|GetCurrentLevelName true))
      (bind (_array_element _array_index) (Utilities|Array|ForEachLoopwithBreak _rooms)
        (:LoopBody
          (Variables|Rooms|SetCurrentIndex _array_index)
          (if (and (Utilities|Enum|Equal(Enum) _array_element _returnvalue_3) (< (Variables|Rooms|GetCurrentIndex) _returnvalue_2))
            (Variables|Rooms|SetNextRoom (Utilities|Array|Get(acopy) (Variables|Rooms|GetRooms) (+ (Variables|Rooms|GetCurrentIndex) 1)))
            (CallFunction|BreakLoop)
            (elif (== (Variables|Rooms|GetCurrentIndex) _returnvalue_2)
              (Variables|Rooms|SetNextRoom "End")
              (CallFunction|BreakLoop))))))
    (:then_1
      (bind _returnvalue_4 (Game|GetCurrentLevelName true))
      (if (not (Utilities|Enum|Equal(Enum) _returnvalue_4 "Start"))
        (CallFunction|GetPlayerStartLocations)
        (CallFunction|SpawnPlayers)))))

(fn ConstructionScript)

(fn SpawnPlayers
  (for _index (range 0 (- (Variables|Players|GetMaxPlayerCount) 1))
    (Variables|Players|SetPlayerIndex _index)
    (for _array_element (Variables|Players|GetPlayerStartArray)
      (if (Utilities|Name|Equal(Name) (Variables|/Script/Engine.PlayerStart|GetPlayerStartTag _array_element) (Utilities|String|StringToName (Utilities|String|ToString(Integer) (Variables|Players|GetPlayerIndex))))
        (Class|GameplayStatics|CreatePlayer (Variables|Players|GetPlayerIndex))
        (bind _returnvalue (Game|SpawnActorfromClass "/Game/Blueprints/Player/BP_PlayerCharacter.BP_PlayerCharacter_C" (Transformation|GetActorTransform _array_element) "AlwaysSpawn" 0 0))
        (Pawn|Possess (Game|GetPlayerController (Variables|Players|GetPlayerIndex)) _returnvalue)
        (Utilities|Array|AddUnique (Variables|Players|GetPlayers) _returnvalue)
        (Variables|/Script/Engine.PlayerController|SetbShowMouseCursor (Game|GetPlayerController (Variables|Players|GetPlayerIndex)) true)
        (Input|SetInputModeGameandUI (Game|GetPlayerController (Variables|Players|GetPlayerIndex)) 0 "DoNotLock" false)))))

(fn GetPlayerStartLocations
  (bind _outactors (Actor|GetAllActorsOfClass "/Script/Engine.PlayerStart"))
  (Variables|Players|SetPlayerStartArray _outactors))

(fn RoomComplete
  (if (Utilities|Enum|Equal(Enum) (Variables|Rooms|GetNextRoom) "End")
    (bind _returnvalue (UserInterface|CreateWidget "/Game/Blueprints/UI/WBP_GameOver.WBP_GameOver_C"))
    (UserInterface|Viewport|AddtoViewport _returnvalue 0)
    (Input|SetInputModeUIOnly (Game|GetPlayerController (Variables|Players|GetPlayerIndex)) _returnvalue "DoNotLock")
    (else
      (Variables|Rooms|SetRoomCleared false)
      (Game|OpenLevel(byName) (Utilities|String|StringToName (Variables|Rooms|GetNextRoom))))))