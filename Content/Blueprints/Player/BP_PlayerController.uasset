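; Player controller that drives the controlled pawn with forward and right axis input along fixed world X and Y axes.
; Both axes call RotateToWASD, which switches the player character to orient rotation to movement unless Attacking is set.
; A MoveToHitLocation function offers SimpleMoveToLocation click-style movement, but nothing here calls it and its zero distance threshold never rejects nearby hits.
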(event Input|AxisEvents|InputAxisMoveForward
  (params (AxisValue :type Float%20%28single-precision%29))
  (bind _returnvalue (Pawn|GetControlledPawn))
  ;[1 1 1] Movement
  (Utilities|IsValid _returnvalue
    (:Is%20Valid
      (Pawn|Input|AddMovementInput _returnvalue "90.000000,0.000000, 0" AxisValue false)
      (CallFunction|RotatetoWASD))))

(event Input|AxisEvents|InputAxisMoveRight
  (params (AxisValue :type Float%20%28single-precision%29))
  (bind _returnvalue (Pawn|GetControlledPawn))
  ;[1 1 1] Movement
  (Utilities|IsValid _returnvalue
    (:Is%20Valid
      (Pawn|Input|AddMovementInput _returnvalue "0.000000,90.000000, 0" AxisValue false)
      (CallFunction|RotatetoWASD))))

(fn ConstructionScript)

(fn MovetoHitLocation
  (params (Hit :type Hit%20Result%20Structure))
  (bind _location (Collision|BreakHitResult Hit))
  (if (>= (Math|Vector|VectorLength (- (Transformation|GetActorLocation (Pawn|GetControlledPawn)) _location)) 0.0) ; Don't move if player clicks too close to pawn
    (AI|Navigation|SimpleMovetoLocation self _location)))

(fn RotatetoWASD
  (bind _returnvalue (Game|GetPlayerCharacter 0))
  (bind _charactermovement (Variables|/Script/Engine.Character|GetCharacterMovement _returnvalue))
  (if (not (Variables|Default|GetAttacking))
    (Utilities|IsValid _returnvalue
      (:Is%20Valid
        (Variables|/Script/Engine.CharacterMovementComponent|SetbOrientRotationToMovement _charactermovement true)
        (Variables|/Script/Engine.CharacterMovementComponent|SetbUseControllerDesiredRotation _charactermovement false)))))