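; A reusable damage component that tracks health for its owning actor, which it destroys when health reaches zero.
; The owner passes in its mesh, health bar widget and health values, and the component checks whether that owner is the player so it can also refresh the player's health.
; Hits spawn screen-projected damage text and briefly tint the mesh red.
; The enemy or ally health bar appears temporarily, lingering longer at low health.
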(event Custom|Take%20Damage%20Via%20Component
  (params (DamageAmount :type Float%20%28single-precision%29))
  (bind _output_get (Variables|Default|SetCurrentHealth (- (Variables|Default|GetCurrentHealth) DamageAmount)))
  (CallFunction|UpdateHealthBar)
  (if (<= _output_get 0.0)
    (Actor|DestroyActor (Variables|Default|GetOwningActor))
    (else
      (bind _returnvalue (CallFunction|SpawnDamageText DamageAmount))
      ;[1 1 1] Red Flash
      (Rendering|Material|SetVectorParameterValueonMaterials (Variables|Default|GetMesh) (Utilities|Name|MakeLiteralName "Overlay") "1.000000,0.100000, 0")
      (Utilities|FlowControl|Delay 0.2)
      (Rendering|Material|SetVectorParameterValueonMaterials (Variables|Default|GetMesh) (Utilities|Name|MakeLiteralName "Overlay") "1.000000,1.000000,1.000000")
      (Utilities|FlowControl|Delay 1.3)
      (Widget|RemovefromParent _returnvalue))))

(event Custom|Setup%20Damagable%20Component
  (params (OwningActor :type Actor%20Object%20Reference) (Mesh :type Mesh%20Component%20Object%20Reference) (HealthBarWidget :type Widget%20Component%20Object%20Reference) (CurrentHealth :type Float%20%28single-precision%29) (MaxHealth :type Float%20%28single-precision%29))
  (Variables|Default|SetOwningActor OwningActor)
  (Variables|Default|SetMesh Mesh)
  (Variables|Default|SetHealthBarWidget HealthBarWidget)
  (Variables|Default|SetCurrentHealth CurrentHealth)
  (Variables|Default|SetMaxHealth MaxHealth)
  (CallFunction|IsPlayer?))

(event Custom|Update%20Health%20Bar
  (if (Variables|Default|GetIsPlayer)
    (Default|CallUpdateHealth (Variables|Default|GetPlayerRef)))
  (Rendering|SetVisibility (Variables|Default|GetHealthBarWidget) true false)
  (Utilities|SetPercent
    (:True
      (Variables|Default|SetHealthBarDelay 5.0))
    (:False
      (Variables|Default|SetHealthBarDelay 2.0)))
  (Utilities|FlowControl|RetriggerableDelay (Variables|Default|GetHealthBarDelay))
  (Rendering|SetVisibility (Variables|Default|GetHealthBarWidget) false false))

(event Custom|UpdateOnLoad
  (params (CurrentHealth :type Float%20%28single-precision%29) (MaxHealth :type Float%20%28single-precision%29))
  (Variables|Default|SetCurrentHealth CurrentHealth)
  (Variables|Default|SetMaxHealth MaxHealth)
  (CallFunction|UpdateHealthBar)
  (Default|CallUpdateHealth (Variables|Default|GetPlayerRef)))

(event EventBeginPlay
  (Rendering|SetVisibility (Variables|Default|GetHealthBarWidget) false false))

(fn SpawnDamageText
  (params (DamageToDisplay :type Float%20%28single-precision%29))
  (bind _returnvalue (UserInterface|CreateWidget "/Game/Blueprints/DamagableComponentSystem/DamageText.DamageText_C" 0 (.ScreenPosition (Class|GameplayStatics|ProjectWorldtoScreen (Game|GetPlayerController 0) (Transformation|GetActorLocation (Variables|Default|GetOwningActor)) false)) DamageToDisplay))
  (UserInterface|Viewport|AddtoViewport _returnvalue 0)
  (return _returnvalue))

(fn IsPlayer?
  (bind _returnvalue (Actor|GetActorOfClass "/Game/Blueprints/Player/BP_PlayerCharacter.BP_PlayerCharacter_C"))
  (if (== _returnvalue (Variables|Default|GetOwningActor))
    (Variables|Default|SetIsPlayer true)
    (Variables|Default|SetPlayerRef _returnvalue)))