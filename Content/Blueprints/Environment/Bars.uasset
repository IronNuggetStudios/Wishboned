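; Environment actor that builds a wall-like grid of bars from one instanced mesh component.
; The Construction Script loops over Length and Height, adding instances in the local XZ plane spaced by Xoffset and Zoffset.
; Each instance gets an unseeded random yaw in half-turn steps to vary the repetition, so the pattern can change on reconstruction.
; The event graph holds no runtime logic.
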(event EventBeginPlay)

(event Collision|EventActorBeginOverlap
  (params (OtherActor :type Actor%20Object%20Reference)))

(event EventTick
  (params (DeltaSeconds :type Float%20%28single-precision%29)))

(fn ConstructionScript
  (for _index (range 0 (- (Variables|Default|GetLength) 1))
    (for _index_2 (range 0 (- (Variables|Default|GetHeight) 1))
      (Components|InstancedStaticMesh|AddInstance (Variables|Default|GetBars) (Math|Transform|MakeTransform (Math|Vector|MakeVector (Math|Conversions|ToFloat(Integer) (* _index (Variables|Default|GetXoffset))) 0.0 (Math|Conversions|ToFloat(Integer) (* _index_2 (Variables|Default|GetZoffset)))) (Math|Rotator|MakeRotator 0.0 0.0 (* (Math|Random|RandomIntegerinRange 0 2) 1.8e+02)))))))