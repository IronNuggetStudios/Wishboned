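; SlimeDaddy is a melee AI enemy that chases the player and splits into several Slime_AI pawns when destroyed.
; It registers with RoomObjective on BeginPlay, while construction wires up its damageable and melee components.
; After a short delay, a timeline's Update drives both chasing and attacking.
; Each attack waits out a cooldown, line-traces, briefly raises an Attacking flag, then calls the melee attack.
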(event EventBeginPlay
  (bind _roomobjective (Variables|Default|GetRoomObjective))
  (Default|SetupRoomObjective _roomobjective true)
  (Default|AddEnemy _roomobjective)
  (Utilities|FlowControl|Delay 1.0)
  (Timeline|Timeline_0 Play
    (:Update
      (Utilities|FlowControl|Sequence
        (:then_0
          (Utilities|ChasePlayer))
        (:then_1
          (Utilities|Attack (Variables|Attack|GetAttackCooldown)))))))

(event EventDestroyed
  (for _index (range 0 (Math|Random|RandomIntegerinRange 2 3))
    (AI|SpawnAIFromClass "/Game/Blueprints/AI/Slime_AI.Slime_AI_C" 0 (Transformation|GetActorLocation) "0, 0, 0" true)))

(fn ConstructionScript
  (Default|SetupDamagableComponent (Variables|Default|GetDamagableComponent) self (Variables|Character|GetMesh) (Variables|Default|GetHealthBar) (Variables|Damagable|GetCurrentHealth) (Variables|Damagable|GetMaxHealth))
  (Default|SetupMeleeAttack (Variables|Default|GetMeleeComponent) (Variables|Default|GetSpawnpoint) (Variables|Attack|GetMeleeRange) (Variables|Attack|GetDamage)))