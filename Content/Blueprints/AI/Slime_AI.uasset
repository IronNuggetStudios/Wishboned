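; Slime enemy AI that registers itself with a room objective, then chases the player and makes melee attacks.
; Construction passes health and attack settings to damageable and melee components.
; After a startup delay, a Timeline's update repeatedly drives AIMoveTo toward the player and a delay-paced attack.
; The attack line-traces, raises an Attacking flag for a short window, then calls the melee component's Attack.
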(event EventBeginPlay
  (bind _roomobjective (Variables|Default|GetRoomObjective))
  (Default|SetupRoomObjective _roomobjective true)
  (Default|AddEnemy _roomobjective)
  (Utilities|FlowControl|Delay 1.0)
  (Timeline|Timeline_0 Play
    (:Update
      (Utilities|FlowControl|Sequence
        (:then_0
          (Utilities|ChasePlayer))
        (:then_1
          (Utilities|Attack (Variables|Attack|GetAttackCooldown)))))))

(fn ConstructionScript
  (Default|SetupDamagableComponent (Variables|Default|GetDamagableComponent) self (Variables|Character|GetMesh) (Variables|Default|GetHealthBar) (Variables|Damagable|GetCurrentHealth) (Variables|Damagable|GetMaxHealth))
  (Default|SetupMeleeAttack (Variables|Default|GetMeleeComponent) (Variables|Default|GetSpawnpoint) (Variables|Attack|GetMeleeRange) (Variables|Attack|GetDamage)))