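; ProjectileSpawningAbility is an attack component that spawns BP_Fireball projectiles.
; A setup event stores the spawn point, damage and scale.
; SpawnProjectile creates a fireball at the spawn point's world location using only its yaw, so the projectile starts level, then applies the scale to its static mesh.
; The stored damage is not passed to the spawned fireball here.
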(event Custom|SetupProjectileSpawningAbility
  (params (Spawnpoint :type Scene%20Component%20Object%20Reference) (Damage :type Float%20%28single-precision%29) (Scale :type Vector))
  (Variables|Default|SetSpawnpoint Spawnpoint)
  (Variables|Default|SetDamage Damage)
  (Variables|Default|SetScale Scale))

(event Custom|SpawnProjectile
  (bind _spawnpoint (Variables|Default|GetSpawnpoint))
  (bind _returnvalue (Game|SpawnActorfromClass "/Game/Blueprints/Projectiles/AllyProjectiles/BP_Fireball.BP_Fireball_C" (Math|Transform|MakeTransform (Transformation|GetWorldLocation _spawnpoint) (Math|Rotator|MakeRotator 0.0 0.0 (.yaw (Transformation|GetWorldRotation _spawnpoint)))) "Undefined" 0 0))
  (Transformation|SetWorldScale3D (Variables|/Game/Blueprints/Projectiles/AllyProjectiles/BaseAllyProjectile.BaseAllyProjectile_C|GetStaticMesh _returnvalue) (Variables|Default|GetScale)))