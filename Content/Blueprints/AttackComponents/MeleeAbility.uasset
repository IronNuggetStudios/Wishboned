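; Melee attack ability that damages whatever damageable actor lies in front of a spawn point within melee range.
; A setup event supplies the spawn point, range and damage.
; LineTrace casts a fixed-length visibility ray along the spawn point's forward vector and stores the hit.
; Attack reuses that stored hit rather than tracing itself, applying damage through the target's DamagableComponent if the hit distance is within range.
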(event Custom|LineTrace
  (bind _spawnpoint (Variables|Default|GetSpawnpoint))
  (bind _returnvalue (Transformation|GetWorldLocation _spawnpoint))
  (bind _outhit (Collision|LineTraceByChannel _returnvalue (+ _returnvalue (* (Math|Vector|GetForwardVector _spawnpoint) 1e+03)) "TraceTypeQuery1" false 0 "None"))
  (Variables|Default|SetHit _outhit))

(event Custom|SetupMeleeAttack
  (params (Spawnpoint :type Scene%20Component%20Object%20Reference) (MeleeRange :type Float%20%28single-precision%29) (Damage :type Float%20%28single-precision%29))
  (Variables|Default|SetSpawnpoint Spawnpoint)
  (Variables|Default|SetMeleeRange MeleeRange)
  (Variables|Default|SetDamage Damage))

(event Custom|Attack
  (bind _hit (Variables|Default|GetHit))
  (bind _returnvalue (Actor|GetComponentbyClass (.hitactor _hit) "/Game/Blueprints/DamagableComponentSystem/DamagableComponent.DamagableComponent_C"))
  (Utilities|IsValid _returnvalue
    (:Is%20Valid
      (if (<= (.distance _hit) (Variables|Default|GetMeleeRange))
        (Default|TakeDamageViaComponent _returnvalue (Variables|Default|GetDamage))))))