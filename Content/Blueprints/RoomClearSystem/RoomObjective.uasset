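; RoomObjective tracks enemies toward clearing a room through counters on BP_Gamemode.
; SetupRoomObjective flags whether it represents an enemy, and AddEnemy increments the game mode's NumberOfEnemies for flagged instances.
; EndPlay decrements that count for enemies, then UpdateRoomCleared sets RoomCleared true only when the count reaches zero.
; The game mode reference is cached on BeginPlay.
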(event Custom|UpdateRoomCleared
  (bind _gamemoderef (Variables|Default|GetGameModeRef))
  (if (== (Variables|/Game/Blueprints/Player/BP_Gamemode.BP_Gamemode_C|GetNumberOfEnemies (Variables|Default|GetGameModeRef)) 0)
    (Variables|/Game/Blueprints/Player/BP_Gamemode.BP_Gamemode_C|SetRoomCleared _gamemoderef true)
    (else
      (Variables|/Game/Blueprints/Player/BP_Gamemode.BP_Gamemode_C|SetRoomCleared _gamemoderef false))))

(event Custom|SetupRoomObjective
  (params (IsEnemy :type Boolean))
  (Variables|Default|SetIsEnemy IsEnemy))

(event Custom|AddEnemy
  (if (Variables|Default|GetIsEnemy)
    (Math|Integer|IncrementInt (Variables|/Game/Blueprints/Player/BP_Gamemode.BP_Gamemode_C|GetNumberOfEnemies (Variables|Default|GetGameModeRef)))))

(event EventBeginPlay
  (bind _asbp_gamemode (Utilities|Casting|CastToBP_Gamemode (Game|GetGameMode)))
  (Variables|Default|SetGameModeRef _asbp_gamemode))

(event EventEndPlay
  (params (EndPlayReason :type EEndPlayReason%20Enum :default "Destroyed"))
  (bind _gamemoderef (Variables|Default|GetGameModeRef))
  (if (Variables|Default|GetIsEnemy)
    (Variables|/Game/Blueprints/Player/BP_Gamemode.BP_Gamemode_C|SetNumberOfEnemies _gamemoderef (- (Variables|/Game/Blueprints/Player/BP_Gamemode.BP_Gamemode_C|GetNumberOfEnemies _gamemoderef) 1))
    (CallFunction|UpdateRoomCleared)))