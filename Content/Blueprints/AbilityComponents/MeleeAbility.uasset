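; MeleeAbility is an ability component that deals melee damage to whatever actor is in front of a spawn point.
; A setup event stores the spawn point, range and damage.
; A separate LineTrace event casts a fixed-length visibility ray along the spawn point's forward vector and caches the hit.
; Attack reads that cached hit and damages the actor through its DamagableComponent if it lies within melee range.
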(event Custom|LineTrace
  (bind _spawnpoint (Variables|Default|GetSpawnpoint))
  (bind _returnvalue (Transformation|GetWorldLocation _spawnpoint))
  (bind (_outhit _returnvalue_2) (Collision|LineTraceByChannel _returnvalue (+ _returnvalue (* (Math|Vector|GetForwardVector _spawnpoint) 1e+03)) "TraceTypeQuery1" false 0 "None"))
  (Variables|Default|SetHitActor _outhit)
  (Variables|Default|SetHit? _returnvalue_2))

(event Custom|SetupMeleeAttack
  (params (Spawnpoint :type Scene%20Component%20Object%20Reference) (MeleeRange :type Float%20%28single-precision%29) (Damage :type Float%20%28single-precision%29))
  (Variables|Default|SetSpawnpoint Spawnpoint)
  (Variables|Default|SetMeleeRange MeleeRange)
  (Variables|Default|SetDamage Damage))

(event Custom|Attack
  (bind _hitactor (Variables|Default|GetHitActor))
  (bind (_bblockinghit _binitialoverlap _time _distance _location _impactpoint _normal _impactnormal _physmat _hitactor_2) (Collision|BreakHitResult _hitactor))
  (bind _returnvalue (Actor|GetComponentbyClass _hitactor_2 "/Game/Blueprints/DamagableComponentSystem/DamagableComponent.DamagableComponent_C"))
  (if (Variables|Default|GetHit?)
    (Utilities|IsValid _returnvalue
      (:Is%20Valid
        (if (<= _distance (Variables|Default|GetMeleeRange))
          (Default|TakeDamageViaComponent _returnvalue (Variables|Default|GetDamage)))))))