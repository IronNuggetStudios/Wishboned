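; Dash ability component that gives its owning character a limited number of quick dashes that recharge over time.
; A dash turns the character toward its last movement input, launches it forward, then halts movement after a very short delay for a burst-like step.
; Each dash spends a charge and, after a pause, starts a looping timer that restores charges one at a time until the maximum is reached.
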(event Custom|Dash
  (bind _owningactor (Variables|Default|GetOwningActor))
  (if (> (Variables|Default|GetDashCount) 0)
    (Transformation|SetActorRotation _owningactor (Math|Conversions|RotationFromXVector (Pawn|Components|PawnMovement|GetLastInputVector (Variables|/Script/Engine.Character|GetCharacterMovement (Variables|Default|GetOwningActor)))))
    (Character|LaunchCharacter _owningactor (* (Transformation|GetActorForwardVector _owningactor) 1e+04) false false)
    (Utilities|FlowControl|Delay 0.03)
    (Variables|Default|SetDashCount (- (Variables|Default|GetDashCount) 1))
    (Components|Movement|StopMovementImmediately (Variables|/Script/Engine.Character|GetCharacterMovement (Variables|Default|GetOwningActor)))
    (Utilities|FlowControl|Delay 1.0)
    (Utilities|Time|SetTimerbyFunctionName 0 "Dash Regen" 1.0 true)))

(event Custom|Setup%20Dash
  (params (OwningActor :type Character%20Object%20Reference) (DashCount :type Integer) (MaxDashes :type Integer))
  (Variables|Default|SetOwningActor OwningActor)
  (Variables|Default|SetDashCount DashCount)
  (Variables|Default|SetMaxDashes MaxDashes))

(event Custom|Dash%20Regen
  (Math|Integer|IncrementInt (Variables|Default|GetDashCount)
    (:%20%20
      (if (not (< (Variables|Default|GetDashCount) (Variables|Default|GetMaxDashes)))
        (Utilities|Time|ClearTimerbyFunctionName 0 "Dash Regen")))))